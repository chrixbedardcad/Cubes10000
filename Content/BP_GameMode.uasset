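; Game mode that shows a debug HUD widget at BeginPlay and maintains its text data: CPU, GPU, FPS, elapsed time and screen resolution.
; Hardware names are read once at startup.
; A Delay on Tick throttles updates to about once per second, advancing the minute:second timer and sampling FPS from frame delta.
; The same Tick fires a DoOnce that captures viewport size, re-armed by Event_Screen_Change.
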(event `self.ReceiveBeginPlay`
  (set `self.CPUBrand` (`KismetTextLibrary.Conv_StringToText` (`KismetStringLibrary.Concat_StrStr` (`HardwareDisplay.GetCPUBrandName`) " (" (`KismetStringLibrary.Conv_IntToString` (`HardwareDisplay.GetCPUCores`)) ") Cores")))
  (set `self.GPUBrand` (`KismetTextLibrary.Conv_StringToText` (`HardwareDisplay.GetGPUBrandName`)))
  (bind _returnvalue (`|CreateWidget` "/Game/HUDFPS.HUDFPS_C" (`GameplayStatics.GetPlayerController` 0)))
  (bind _output_get (set `self.Hud_ref` _returnvalue))
  (`UserWidget.AddToViewport` _output_get 0))

(event `Event_Screen_Change`
  (bind (_sizex _sizey) (`PlayerController.GetViewportSize` (`GameplayStatics.GetPlayerController` 0)))
  (goto _label :!via `Reset`))

(event `self.ReceiveTick`
  (params (DeltaSeconds :type "Float (single-precision)"))
  (bind (_sizex _sizey) (`PlayerController.GetViewportSize` (`GameplayStatics.GetPlayerController` 0)))
  (`KismetSystemLibrary.Delay` 1.0)
  (if (< (`self.TimeSec`) 9)
    (set `self.TimerText` (`KismetTextLibrary.Conv_StringToText` (`KismetStringLibrary.Concat_StrStr` (`KismetStringLibrary.Conv_IntToString` (`self.TimeMin`)) ":" "0" (`KismetStringLibrary.Conv_IntToString` (`self.TimeSec`)))))
    (else
      (set `self.TimerText` (`KismetTextLibrary.Conv_StringToText` (`KismetStringLibrary.Concat_StrStr` (`KismetStringLibrary.Conv_IntToString` (`self.TimeMin`)) ":" (`KismetStringLibrary.Conv_IntToString` (`self.TimeSec`)))))))
  (set `self.FPSUpdate` (`KismetTextLibrary.Conv_IntToText` (`KismetMathLibrary.FTrunc` (/ 1.0 DeltaSeconds))))
  (set `self.TimeSec` (+ (`self.TimeSec`) 1))
  (if (> (`self.TimeSec`) 59)
    (set `self.TimeMin` (+ (`self.TimeMin`) 1))
    (set `self.TimeSec` 0)
    (else
      (`/Engine/EditorBlueprintResources/StandardMacros.DoOnce` false :!label _label
        (:`Completed`
          (set `self.ScreenRez` (`KismetTextLibrary.Conv_StringToText` (`KismetStringLibrary.Concat_StrStr` (`KismetStringLibrary.Conv_IntToString` _sizex) " x " (`KismetStringLibrary.Conv_IntToString` _sizey)))))))))

(fn `UserConstructionScript`)